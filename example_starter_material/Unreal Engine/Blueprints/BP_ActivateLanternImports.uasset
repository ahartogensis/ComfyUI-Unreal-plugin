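; Level actor that switches on Hyper3D object imports for a lantern setup while it is in play.
; On BeginPlay it turns off splat-driven box placement, activates imports, and configures the Hyper3D Objects subsystem with instance count and box size from its variables.
; It uses its own location as the placement reference and sets a fixed object scale and fade-in duration.
; EndPlay deactivates the imports.
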(event `self.ReceiveBeginPlay`
  (bind _returnvalue (subsystem `Hyper3DObjectsSubsystem`))
  (set `Hyper3DObjectsSubsystem.bDrivePlacementBoxFromSplat` false _returnvalue)
  (`Hyper3DObjectsSubsystem.ActivateObjectImports` _returnvalue)
  (`Hyper3DObjectsSubsystem.SetTotalInstances` _returnvalue (`self.In Total Instances`))
  (`Hyper3DObjectsSubsystem.SetReferenceLocation` _returnvalue (`self.K2_GetActorLocation`))
  (set `Hyper3DObjectsSubsystem.BoxSize` (`self.In Box Size`) _returnvalue)
  (`Hyper3DObjectsSubsystem.SetHyper3DObjectScale` _returnvalue 80.0)
  (`Hyper3DObjectsSubsystem.SetHyper3DObjectFadeInDuration` _returnvalue 4.0))

(event `self.ReceiveEndPlay`
  (params (EndPlayReason :type "EEndPlayReason Enum" :default "Destroyed"))
  (`Hyper3DObjectsSubsystem.DeactivateObjectImports` (subsystem `Hyper3DObjectsSubsystem`)))

(fn `UserConstructionScript`)