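; Actor that switches on Hyper3D object imports, presumably for lanterns given its name, for as long as it is in play.
; On BeginPlay it passes its location as the reference point and its InTotalInstances count to the Hyper3DObjects subsystem, activates imports, then triggers an update from splat dimensions.
; On EndPlay it deactivates the imports, leaving all import logic to the subsystem.
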(event `self.ReceiveBeginPlay`
  (bind _returnvalue (subsystem `Hyper3DObjectsSubsystem`))
  (`Hyper3DObjectsSubsystem.SetReferenceLocation` _returnvalue (`self.K2_GetActorLocation`))
  (`Hyper3DObjectsSubsystem.ActivateObjectImports` _returnvalue)
  (`Hyper3DObjectsSubsystem.SetTotalInstances` _returnvalue (`self.In Total Instances`))
  (`Hyper3DObjectsSubsystem.SetReferenceLocation` _returnvalue (`self.K2_GetActorLocation`))
  (`Hyper3DObjectsSubsystem.UpdateFromSplatDimensions` _returnvalue))

(event `self.ReceiveEndPlay`
  (params (EndPlayReason :type "EEndPlayReason Enum" :default "Destroyed"))
  (`Hyper3DObjectsSubsystem.DeactivateObjectImports` (subsystem `Hyper3DObjectsSubsystem`)))

(fn `UserConstructionScript`)